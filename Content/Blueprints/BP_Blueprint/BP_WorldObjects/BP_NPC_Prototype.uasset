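; Prototype NPC that takes hand-ins of two "Russekort" card pieces from the player, BP_Emmi.
; Tick, active only for pinch levels 3 to 5, toggles readiness and InfoText by player distance, placing the text midway toward the camera and turning it to face it.
; CardCollection checks the player's inventory for each piece in order, setting progress flags and updating InfoText.
; Once Done is set, Tick hides the text.
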(event Custom|CardCollection
  ;[1 1 1] Collect Cards
  (if (Variables|Default|GetReady)
    (bind _asbp_emmi (Utilities|Casting|CastToBP_Emmi (Game|Player|GetPlayerPawn 0)))
    (if (Variables|Default|GetFirstCard)
      (bind _found (Default|CheckIteminInventory _asbp_emmi "Russekort2"))
      (if _found
        (Rendering|Components|TextRender|SetText (Variables|Default|GetInfoText) (Utilities|Text|ToText(String) "Card complete"))
        (Variables|Default|SetSecondCard true)
        (else
          (Rendering|Components|TextRender|SetText (Variables|Default|GetInfoText) (Utilities|Text|ToText(String) "Last piece missing"))))
      (else
        (bind _found_2 (Default|CheckIteminInventory _asbp_emmi "Russekort1"))
        (if _found_2
          (Rendering|Components|TextRender|SetText (Variables|Default|GetInfoText) (Utilities|Text|ToText(String) "One more part. Does not seem like it is in this dream..."))
          (Variables|Default|SetFirstCard true)
          (else
            (Rendering|Components|TextRender|SetText (Variables|Default|GetInfoText) (Utilities|Text|ToText(String) "Find the missing pieces"))))))))

(event Collision|EventActorBeginOverlap
  (params (OtherActor :type Actor%20Object%20Reference)))

(event EventBeginPlay
  ;[1 1 1] Init
  (bind _asbp_emmi (Utilities|Casting|CastToBP_Emmi (Game|Player|GetPlayerPawn 0)))
  (Variables|Default|SetPlayer _asbp_emmi))

(event EventTick
  (params (DeltaSeconds :type Float%20%28single-precision%29))
  (bind _returnvalue (Transformation|GetActorLocation))
  (bind _returnvalue_2 (Transformation|GetActorLocation))
  (bind _returnvalue_3 (Game|GetPlayerCameraManager 0))
  (bind _player (Variables|Default|GetPlayer))
  (bind _infotext (Variables|Default|GetInfoText))
  (bind _returnvalue_4 (Camera|GetCameraLocation _returnvalue_3))
  (bind _returnvalue_5 (Camera|GetCameraLocation _returnvalue_3))
  (bind _pinchmanager (Variables|/Game/Blueprints/BP_Blueprint/BP_Player/BP_Emmi.BP_Emmi_C|GetPinchManager _player))
  (bind _returnvalue_6 (Math|Vector|MakeVector (.x _returnvalue) (.y _returnvalue) (.z _returnvalue_4)))
  (bind _currentlevel (Variables|/Game/Blueprints/BP_Blueprint/BP_Player/BP_PinchManager.BP_PinchManager_C|GetcurrentLevel _pinchmanager))
  (bind _returnvalue_7 (- _returnvalue_5 _returnvalue_6))
  (bind _returnvalue_8 (* _returnvalue_7 0.5))
  (bind _returnvalue_9 (+ _returnvalue_6 _returnvalue_8))
  (bind _returnvalue_10 (Math|Rotator|FindLookatRotation _returnvalue_2 _returnvalue_9))
  ;[1 1 1] Check if player is close and rotate text to camera
  (if (and (Variables|Default|GetReady) (not (Variables|Rendering|GetbHidden)))
    (Development|PrintString "Press F to hand in card" false true "(R=0.000000,G=0.660000,B=1.000000,A=1.000000)" 0.01 "npc")
    (Default|ChangeText (Variables|/Game/Blueprints/BP_Blueprint/BP_Player/BP_Emmi.BP_Emmi_C|GetUI (Variables|Default|GetPlayer)) "Press F to hand in card"))
  (if (and (>= _currentlevel 3) (< _currentlevel 6))
    (if (Variables|Default|GetDone)
      (Utilities|FlowControl|DoOnce false
        (:Completed
          (Development|SetHiddeninGame _infotext true false)))
      (elif (< (Variables|Default|GetDistance) (Math|Vector|Distance(Vector) (Transformation|GetActorLocation (Variables|Default|GetPlayer)) (Transformation|GetActorLocation self)))
        (Development|SetHiddeninGame _infotext true false)
        (Variables|Default|SetReady false)
        (else
          (Development|SetHiddeninGame (Variables|Default|GetInfoText) false false)
          (Variables|Default|SetReady true)
          (Collision|LineTraceByChannel _returnvalue_5 _returnvalue_6 "TraceTypeQuery1" false 0 "None")
          (Transformation|SetWorldLocation (Variables|Default|GetInfoText) _returnvalue_9 false false)
          (Transformation|SetWorldRotation (Variables|Default|GetInfoText) (Math|Rotator|MakeRotator (.roll _returnvalue_10) (.pitch (Transformation|GetWorldRotation (Variables|Default|GetInfoText))) (.yaw _returnvalue_10)) false false))))))

(fn ConstructionScript)