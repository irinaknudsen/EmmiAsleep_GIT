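; BP_ButtonM is an interactable world button that toggles linked doors when the player holds a required item.
; BeginPlay caches BP_Emmi and its inspect range; Tick swaps the button's material to red within range, blue beyond.
; Pressed checks the player's inventory, then dispatches on Index, with case 0 calling Door and others printing.
; Door toggles visibility and collision on DoorActors, also switching physics simulation on the button's own mesh.
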(event Custom|Pressed
  (bind _itemneeded (Variables|Default|GetitemNeeded))
  ;[1 1 1] Activate different functions as button is pressed
  (bind _found (Default|CheckIteminInventory (Variables|Default|Getplayer) _itemneeded))
  (if (and (Utilities|Enum|NotEqual(Enum) _itemneeded "X") _found)
    (switch int (Variables|Default|Getindex)
      (:Default
        (Development|PrintString "Button Pressed!"))
      (:0
        (CallFunction|Door)))
    (else
      (Development|PrintString "ReqiuredItemNotInInventory"))))

(event EventBeginPlay
  ;[1 1 1] Get Interact Distance from player blueprint
  (bind _asbp_emmi (Utilities|Casting|CastToBP_Emmi (Game|Player|GetPlayerPawn 0)))
  (Variables|Default|SetInteractDistance (Math|Conversions|ToFloat(Integer) (Variables|/Game/Blueprints/BP_Blueprint/BP_Player/BP_Emmi.BP_Emmi_C|GetInspectRange _asbp_emmi)))
  (Variables|Default|Setplayer _asbp_emmi))

(event Collision|EventActorBeginOverlap
  (params (OtherActor :type Actor%20Object%20Reference)))

(event EventTick
  (params (DeltaSeconds :type Float%20%28single-precision%29))
  ;[1 1 1] Updating material based on distance to player ( red color if player is close enough to interact)
  (Math|Float|CompareFloat (Math|Vector|Distance(Vector) (Transformation|GetActorLocation (Game|Player|GetPlayerPawn 0)) (Transformation|GetActorLocation self)) (Variables|Default|GetInteractDistance)
    (:>
      (Rendering|Material|SetMaterial (Variables|Debug|GetStaticMeshComponent) 0 "/Game/Assets/Materials/M_Material/M_Jeldrik/MI_Solid_Blue.MI_Solid_Blue"))
    (:<
      (Rendering|Material|SetMaterial (Variables|Debug|GetStaticMeshComponent) 0 "/Game/Assets/Materials/M_Material/M_Jeldrik/M_Solid_Red.M_Solid_Red"))))

(fn ConstructionScript)

(fn Door
  (for _array_element (Variables|Default|GetdoorActors)
    (if (Variables|/Script/Engine.Actor|GetbHidden _array_element)
      (Rendering|SetActorHiddenInGame _array_element false)
      (Collision|SetActorEnableCollision _array_element true)
      (Physics|SetSimulatePhysics (Variables|Debug|GetStaticMeshComponent) true)
      (else
        (Rendering|SetActorHiddenInGame _array_element true)
        (Collision|SetActorEnableCollision _array_element false)
        (Physics|SetSimulatePhysics (Variables|Debug|GetStaticMeshComponent) false)))))