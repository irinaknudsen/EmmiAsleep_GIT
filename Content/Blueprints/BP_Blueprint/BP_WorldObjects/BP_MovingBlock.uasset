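; BP_MovingBlock is a pushable world block that the player (BP_Emmi) shoves in front of a door.
; Tick checks player distance to toggle the InfoText prompt and Ready, then fires a one-shot push if Moving is set.
; The push plays a timeline along X, disabling input and aiming the player's view at the block until Done.
; A separate Move event offsets the block in X and Y by button-mash progress.
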(event Custom|Move
  (bind _player (Variables|Default|GetPlayer))
  (bind _movedistance (Variables|Default|GetMoveDistance))
  (bind _mashgoal (Variables|/Game/Blueprints/BP_Blueprint/BP_Player/BP_Emmi.BP_Emmi_C|GetMashGoal _player))
  (bind _mashcounter (Variables|/Game/Blueprints/BP_Blueprint/BP_Player/BP_Emmi.BP_Emmi_C|GetMashCounter _player))
  (bind _returnvalue (/ _mashcounter _mashgoal))
  (bind _returnvalue_2 (* _movedistance _returnvalue))
  ;[1 1 1] Move with Mashing
  (if (Variables|Default|GetReady)
    (Physics|SetSimulatePhysics (Variables|Debug|GetStaticMeshComponent) false)
    (Transformation|SetActorLocation (+ (Variables|Default|GetStartPos) (Math|Vector|MakeVector _returnvalue_2 _returnvalue_2 0.0)) false false)))

(event Custom|MoveDrrawer
  (bind _player (Variables|Default|GetPlayer))
  ;[1 1 1] Pushing block infront of door
  (if (and (Variables|Default|GetReady) (not (Variables|Default|GetDone)))
    (Variables|Default|SetStartPos (Transformation|GetActorLocation self))
    (Input|DisableInput (Variables|Default|GetPlayer) 0)
    (Physics|SetSimulatePhysics (Variables|Debug|GetStaticMeshComponent) false)
    (bind _pos (Timeline|Timeline_0 PlayFromStart)
      (:Update
        (Transformation|SetActorLocation (+ (Variables|Default|GetStartPos) (Math|Vector|MakeVector _pos 0.0 0.0)) false false)
        (Pawn|SetControlRotation (Pawn|GetController _player) (Math|Rotator|FindLookatRotation (Transformation|GetActorLocation _player) (Transformation|GetActorLocation self))))
      (:Finished
        (Input|EnableInput (Variables|Default|GetPlayer) 0)
        (Physics|SetSimulatePhysics (Variables|Debug|GetStaticMeshComponent) false)
        (Development|SetHiddeninGame (Variables|Default|GetInfoText) true false)
        (Variables|Default|SetDone true)
        (Variables|Default|SetMoving false)))))

(event EventBeginPlay
  ;[1 1 1] Init
  (bind _asbp_emmi (Utilities|Casting|CastToBP_Emmi (Game|Player|GetPlayerPawn 0)))
  (Variables|Default|SetPlayer _asbp_emmi)
  (Variables|Default|SetStartPos (Transformation|GetActorLocation self)))

(event EventTick
  (params (DeltaSeconds :type Float%20%28single-precision%29))
  (bind _infotext (Variables|Default|GetInfoText))
  ;[1 1 1] Determine if player is in range
  (if (Variables|Default|GetDone)
    (Utilities|FlowControl|DoOnce false
      (:Completed
        (Development|SetHiddeninGame _infotext true false)))
    (elif (< (Variables|Default|GetDistance) (Math|Vector|Distance(Vector) (Transformation|GetActorLocation (Variables|Default|GetPlayer)) (Transformation|GetActorLocation self)))
      (Development|SetHiddeninGame _infotext true false)
      (Variables|Default|SetReady false)
      (else
        (Development|SetHiddeninGame (Variables|Default|GetInfoText) false false)
        (Variables|Default|SetReady true)
        (if (Variables|Default|GetMoving)
          (Utilities|FlowControl|DoOnce false
            (:Completed
              (CallFunction|MoveDrrawer))))))))

(fn ConstructionScript)