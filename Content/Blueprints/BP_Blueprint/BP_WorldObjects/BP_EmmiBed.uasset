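; BP_EmmiBed is a bed world object apparently meant to let the player character BP_Emmi sleep, but it is currently inert.
; BeginPlay, Tick, EnterBed and the construction script are empty, and all the logic sits in disconnected nodes.
; Those leftovers check SleepTrigger overlap and PinchManager level to set Emmi's CanSleep and UI prompt, call Pinch on entering, and destroy the trigger.
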(event Custom|EnterBed
  ;[1 1 1] Handle Player entering the Bed
)

(event EventBeginPlay)

(event EventTick
  (params (DeltaSeconds :type Float%20%28single-precision%29))
  ;[1 1 1] Checking if Emmi enters Bed
)

(event Input|KeyboardEvents|F
  (params (Key :type Key%20Structure :default "None")))

(fn ConstructionScript)