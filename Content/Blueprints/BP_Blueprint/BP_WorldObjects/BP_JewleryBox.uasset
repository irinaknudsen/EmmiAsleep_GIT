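; BP_JewleryBox is an interactive jewelry box world object with a hinged lid and a spinning heart charm.
; Input is enabled for the first player controller on BeginPlay.
; Tick continuously rotates the charm around yaw by the Rotate variable.
; The OpenBox event plays the Open timeline, which tilts the lid up to an angle on roll and sets IsOpen.
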(event Custom|OpenBox
  ;[1 1 1] åbna låkke
  (bind _open (Timeline|open Play)
    (:Update
      (Transformation|SetRelativeRotation (Variables|Default|GetTop_Box) (Math|Rotator|MakeRotator (* _open 6e+01) 0.0 0.0) false false)
      (Variables|Default|SetisOpen true))))

(event EventBeginPlay
  ;[1 1 1] Må hame denne for å enable input!!!!!!!!!!!!!!!
  (Input|EnableInput (Game|GetPlayerController 0)))

(event EventTick
  (params (DeltaSeconds :type Float%20%28single-precision%29))
  ;[1 1 1] Rotating Heart
  (Transformation|AddRelativeRotation (Variables|Default|GetTopBox_Charm) (Math|Rotator|MakeRotator 0.0 0.0 (Variables|Default|Getrotate)) false false))

(fn ConstructionScript)