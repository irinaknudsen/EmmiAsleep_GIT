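; BP_SaveManager defines saving and restoring of the state of actors tagged "pinch" through an F_PinchSaveClass save game.
; CreateSaveGame records each actor's transform (location, rotation), visibility, tick and collision state in maps keyed by actor reference.
; LoadSaveGame reads the slot and reapplies those values to the stored actors.
; SaveLevel and LoadLevel are empty events; the slot save and load calls are disconnected, so neither runs.
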(event Custom|LoadLevel
  ;[1 1 1] Loading save game
)

(event Custom|SaveLevel
  ;[1 1 1] Saving save game
)

(fn CreateSaveGame
  (bind _outactors (Actor|GetAllActorswithTag "pinch"))
  (bind _returnvalue (SaveGame|CreateSaveGameObject "/Game/Blueprints/BP_Blueprint/BP_Player/F_PinchSaveClass.F_PinchSaveClass_C"))
  (for _array_element _outactors
    (Utilities|Array|Add (Variables|/Game/Blueprints/BP_Blueprint/BP_Player/F_PinchSaveClass.F_PinchSaveClass_C|GetActors _returnvalue) _array_element)
    (Utilities|Map|Add (Variables|/Game/Blueprints/BP_Blueprint/BP_Player/F_PinchSaveClass.F_PinchSaveClass_C|GetLocations _returnvalue) _array_element (Transformation|GetActorLocation _array_element))
    (Utilities|Map|Add (Variables|/Game/Blueprints/BP_Blueprint/BP_Player/F_PinchSaveClass.F_PinchSaveClass_C|GetRotations _returnvalue) _array_element (Transformation|GetActorRotation _array_element))
    (Utilities|Map|Add (Variables|/Game/Blueprints/BP_Blueprint/BP_Player/F_PinchSaveClass.F_PinchSaveClass_C|GetHidden _returnvalue) _array_element (Variables|/Script/Engine.Actor|GetbHidden _array_element))
    (Utilities|Map|Add (Variables|/Game/Blueprints/BP_Blueprint/BP_Player/F_PinchSaveClass.F_PinchSaveClass_C|GetTick _returnvalue) _array_element (Class|Actor|IsActorTickEnabled _array_element))
    (Utilities|Map|Add (Variables|/Game/Blueprints/BP_Blueprint/BP_Player/F_PinchSaveClass.F_PinchSaveClass_C|GetCollision _returnvalue) _array_element (Collision|GetActorEnableCollision _array_element)))
  (return _returnvalue))

(fn LoadSaveGame
  (params (slotName :type String))
  (bind _returnvalue (SaveGame|LoadGamefromSlot slotName))
  (bind _asf_pinch_save_class (Utilities|Casting|CastToF_PinchSaveClass _returnvalue))
  (for _array_element (Variables|/Game/Blueprints/BP_Blueprint/BP_Player/F_PinchSaveClass.F_PinchSaveClass_C|GetActors _asf_pinch_save_class)
    (LocalVariables|SetAc _array_element)
    (Transformation|SetActorLocationAndRotation _array_element (.Value (Utilities|Map|Find (Variables|/Game/Blueprints/BP_Blueprint/BP_Player/F_PinchSaveClass.F_PinchSaveClass_C|GetLocations _asf_pinch_save_class) _array_element)) (.Value (Utilities|Map|Find (Variables|/Game/Blueprints/BP_Blueprint/BP_Player/F_PinchSaveClass.F_PinchSaveClass_C|GetRotations _asf_pinch_save_class) _array_element)))
    (Rendering|SetActorHiddenInGame _array_element (.Value (Utilities|Map|Find (Variables|/Game/Blueprints/BP_Blueprint/BP_Player/F_PinchSaveClass.F_PinchSaveClass_C|GetHidden _asf_pinch_save_class) (LocalVariables|GetAc))))
    (Actor|Tick|SetActorTickEnabled _array_element (.Value (Utilities|Map|Find (Variables|/Game/Blueprints/BP_Blueprint/BP_Player/F_PinchSaveClass.F_PinchSaveClass_C|GetTick _asf_pinch_save_class) (LocalVariables|GetAc))))
    (Collision|SetActorEnableCollision _array_element (.Value (Utilities|Map|Find (Variables|/Game/Blueprints/BP_Blueprint/BP_Player/F_PinchSaveClass.F_PinchSaveClass_C|GetCollision _asf_pinch_save_class) (LocalVariables|GetAc))))))