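; Level manager that switches between six levels by showing or hiding actors tagged "LevelN" and toggling their collision.
; Actors also tagged with an adjacent level number are skipped when hiding.
; LoadLevel snapshots BP_Emmi's inventory for LoadInv to restore, then, except for level 1, moves the player to a given transform or the cached PlayerStart.
; CreateLevelSafe writes a per-level save slot, guarded by a press-again confirmation.
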(event EventBeginPlay
  (bind _outactors (Actor|GetAllActorswithTag "playerStart"))
  (bind _asplayer_start (Utilities|Casting|CastToPlayerStart (Utilities|Array|Get(acopy) _outactors)))
  (Variables|Default|SetplayerStart _asplayer_start)
  (Variables|Default|SetstartPos (Transformation|GetActorLocation (Variables|Default|GetplayerStart)))
  (Variables|Default|SetstartRot (Transformation|GetActorRotation (Variables|Default|GetplayerStart))))

(fn CreateLevelSafe
  (params (Level :type Integer))
  (if (Variables|Default|Getsafety)
    (Utilities|FlowControl|DoOnce false :!label _label
      (:Completed
        (Development|PrintString "Press again to safe")
        (Variables|Default|Setsafety false)))
    (else
      (bind _asbp_emmi (Utilities|Casting|CastToBP_Emmi (Game|Player|GetPlayerPawn 0)))
      (bind _gamesave (Default|CreateSaveGame (Variables|/Game/Blueprints/BP_Blueprint/BP_Player/BP_Emmi.BP_Emmi_C|GetSaveManager1 _asbp_emmi)))
      (SaveGame|SaveGametoSlot _gamesave (Utilities|String|Append "Level" (Utilities|String|ToString(Integer) Level)))
      (Variables|Default|Setsafety true)
      (goto _label Reset))))

(fn EnableLevelObject
  (params (Level :type Integer))
  (bind _outactors (Actor|GetAllActorswithTag (Utilities|String|StringToName (Utilities|String|Append "Level" (Utilities|String|ToString(Integer) Level)))))
  (for _array_element _outactors
    (Rendering|SetActorHiddenInGame _array_element false)
    (Collision|SetActorEnableCollision _array_element true)))

(fn DisabeLevelObject
  (params (Level :type Integer))
  (for _index (range 1 6)
    (if (not (== Level _index))
      (bind _outactors (Actor|GetAllActorswithTag (Utilities|String|StringToName (Utilities|String|Append "Level" (Utilities|String|ToString(Integer) _index)))))
      (for _array_element _outactors
        (if (and (not (Actor|ActorHasTag _array_element (Utilities|String|StringToName (Utilities|String|Append "Level" (Utilities|String|ToString(Integer) (- _index 1)))))) (not (Actor|ActorHasTag _array_element (Utilities|String|StringToName (Utilities|String|Append "Level" (Utilities|String|ToString(Integer) (+ _index 1)))))))
          (Rendering|SetActorHiddenInGame _array_element true)
          (Collision|SetActorEnableCollision _array_element false))))))

(fn LoadLevel
  (params (Level :type Integer) (LoadWithPos :type Boolean) (Loading%20pos :type Vector) (Loading%20rot :type Rotator))
  (CallFunction|EnableLevelObject Level)
  (CallFunction|DisabeLevelObject Level)
  (CallFunction|SaveInv)
  (if (not (== Level 1))
    (if LoadWithPos
      ;[1 1 1] Reset player to provided pos and rot
      (Transformation|SetActorLocation (Game|Player|GetPlayerPawn 0) Loading%20pos false false)
      (Pawn|SetControlRotation (Game|GetPlayerController 0) Loading%20rot)
      (else
        ;[1 1 1] Reset player to starting Pos and Rot
        (Transformation|SetActorLocation (Game|Player|GetPlayerPawn 0) (Variables|Default|GetstartPos) false false)
        (Pawn|SetControlRotation (Game|GetPlayerController 0) (Variables|Default|GetstartRot))))))

(fn SaveInv
  (bind _asbp_emmi (Utilities|Casting|CastToBP_Emmi (Game|Player|GetPlayerPawn 0)))
  (Variables|Default|SetinventorySave (Variables|/Game/Blueprints/BP_Blueprint/BP_Player/BP_Emmi.BP_Emmi_C|GetCollectedItems _asbp_emmi)))

(fn LoadInv
  (bind _asbp_emmi (Utilities|Casting|CastToBP_Emmi (Game|Player|GetPlayerPawn 0)))
  (Variables|/Game/Blueprints/BP_Blueprint/BP_Player/BP_Emmi.BP_Emmi_C|SetCollectedItems _asbp_emmi (Variables|Default|GetinventorySave)))