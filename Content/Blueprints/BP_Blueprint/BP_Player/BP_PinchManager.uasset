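; Pinch manager that drives level progression: on a Pinch event it checks whether the current level's goal is met.
; PinchCheck switches on CurrentLevel to test state on the Emmi pawn or tag-found block, jewelry box and card-collector NPC.
; Success loads the next level through LevelManager, while failure reloads it, and five failures or passing the last level fades the camera and quits.
; Tick removes the door at level 6, and key 3 is a debug level skip.
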(event Custom|Pinch
  (bind _currentlevel (Variables|Default|GetcurrentLevel))
  ;[1 1 1] Pinch
  (bind _conditionsmet (CallFunction|PinchCheck))
  (if _conditionsmet
    (Math|Integer|IncrementInt _currentlevel
      (:%20%20
        (if (Variables|Default|GetskipBoxLevel)
          (Math|Integer|IncrementInt (Variables|Default|GetcurrentLevel)
            (:%20%20
              (Variables|Default|SetskipBoxLevel false))))
        (if (>= _currentlevel 7)
          (CallFunction|WinGame)
          (Utilities|FlowControl|Delay 1.0)
          (CameraFades|StartCameraFade (Game|GetPlayerCameraManager 0) 0.0 1.0 3.0 "(R=0.152812,G=0.929167,B=0.268328,A=1.000000)" false false)
          (Utilities|FlowControl|Delay 3.0)
          (Game|QuitGame 0 "Quit" false)
          (else
            (Default|LoadLevel (Variables|Default|GetLevelManager) (Variables|Default|GetcurrentLevel) false "0, 0, 0" "0, 0, 0")
            (Variables|Default|SetpinchCounter 0)
            (Development|PrintString "Level completed")))))
    (else
      (Development|PrintString "Pinch failed reset level and increase pinch counter")
      (Default|LoadInv (Variables|Default|GetLevelManager))
      (Default|LoadLevel (Variables|Default|GetLevelManager) (Variables|Default|GetcurrentLevel) false "0, 0, 0" "0, 0, 0")
      (Math|Integer|IncrementInt (Variables|Default|GetpinchCounter)
        (:%20%20
          (if (>= (Variables|Default|GetpinchCounter) 5)
            (CallFunction|LooseGame)
            (Utilities|FlowControl|Delay 1.0)
            (CameraFades|StartCameraFade (Game|GetPlayerCameraManager 0) 0.0 1.0 3.0 "(R=0.929167,G=0.006671,B=0.000000,A=1.000000)" false false)
            (Utilities|FlowControl|Delay 3.0)
            (Game|QuitGame 0 "Quit" false)))))))

(event EventTick
  (params (DeltaSeconds :type Float%20%28single-precision%29))
  (if (== (Variables|Default|GetcurrentLevel) 6)
    (Utilities|FlowControl|DoOnce false
      (:Completed
        (Actor|DestroyActor (Variables|Default|Getdoor))
        (Actor|DestroyActor (Variables|Default|GetdoorHandle))))))

(event EventBeginPlay
  ;[1 1 1] Init
  (bind _outactors (Actor|GetAllActorswithTag "door"))
  (Variables|Default|Setdoor (Utilities|Array|Get(acopy) _outactors))
  (Variables|Default|SetdoorHandle (Utilities|Array|Get(acopy) _outactors 1))
  (bind _asbp_emmi (Utilities|Casting|CastToBP_Emmi (Game|Player|GetPlayerPawn 0)))
  (Variables|Default|SetSaveManager (Variables|/Game/Blueprints/BP_Blueprint/BP_Player/BP_Emmi.BP_Emmi_C|GetSaveManager1 _asbp_emmi))
  (Variables|Default|SetLevelManager (Variables|/Game/Blueprints/BP_Blueprint/BP_Player/BP_Emmi.BP_Emmi_C|GetLevelManager _asbp_emmi))
  (Variables|Default|Setemmi _asbp_emmi)
  (if (not (Variables|Default|GetCreateLevel))
    (Default|LoadLevel (Variables|/Game/Blueprints/BP_Blueprint/BP_Player/BP_Emmi.BP_Emmi_C|GetLevelManager _asbp_emmi) (Variables|Default|GetcurrentLevel) false "0, 0, 0" "0, 0, 0")))

(event Input|KeyboardEvents|3
  (params (Key :type Key%20Structure :default "None"))
  ;[1 1 1] Debug to skip to 3rd level
  (:Pressed
    (Default|LoadLevel (Variables|Default|GetLevelManager) 4 false "0, 0, 0" "0, 0, 0")
    (Variables|Default|SetcurrentLevel 4)))

(fn PinchCheck
  (switch int (Variables|Default|GetcurrentLevel)
    (:Default
      _)
    (:0
      _)
    (:1
      (if (Variables|/Game/Blueprints/BP_Blueprint/BP_Player/BP_Emmi.BP_Emmi_C|Getslept (Variables|Default|Getemmi))
        (return true)
        (else
          (return false))))
    (:2
      (bind _completed (CallFunction|Level2Check))
      (return _completed))
    (:3
      (bind _completed_2 (CallFunction|Level1Check))
      (return _completed_2))
    (:4
      (bind _completed_3 (CallFunction|Level3Check))
      (return _completed_3))
    (:5
      (bind _completed_4 (CallFunction|Level4Check))
      (return _completed_4)))
  (return false))

(fn Level1Check
  (bind _outactors (Actor|GetAllActorswithTag "level1cond1"))
  (bind _asbp_moving_block (Utilities|Casting|CastToBP_MovingBlock (Utilities|Array|Get(acopy) _outactors)))
  (if (Variables|/Game/Blueprints/BP_Blueprint/BP_WorldObjects/BP_MovingBlock.BP_MovingBlock_C|GetDone _asbp_moving_block)
    (return true)
    (else
      (return false))))

(fn Level2Check
  (bind _asbp_emmi (Utilities|Casting|CastToBP_Emmi (Game|Player|GetPlayerPawn 0)))
  (bind _found (Default|CheckIteminInventory _asbp_emmi "key1"))
  (bind _outactors (Actor|GetAllActorswithTag "jewleryBox"))
  (bind _asbp_jewlery_box (Utilities|Casting|CastToBP_JewleryBox (Utilities|Array|Get(acopy) _outactors)))
  (return (and (Variables|/Game/Blueprints/BP_Blueprint/BP_WorldObjects/BP_JewleryBox.BP_JewleryBox_C|GetisOpen _asbp_jewlery_box) _found)))

(fn Level3Check
  (bind _outactors (Actor|GetAllActorswithTag "card collector"))
  (bind _asbp_npc_prototype (Utilities|Casting|CastToBP_NPC_Prototype (Utilities|Array|Get(acopy) _outactors)))
  (if (Variables|/Game/Blueprints/BP_Blueprint/BP_WorldObjects/BP_NPC_Prototype.BP_NPC_Prototype_C|GetFirstCard _asbp_npc_prototype)
    (return true)
    (else
      (return false))))

(fn Level4Check
  (bind _outactors (Actor|GetAllActorswithTag "card collector"))
  (bind _asbp_npc_prototype (Utilities|Casting|CastToBP_NPC_Prototype (Utilities|Array|Get(acopy) _outactors)))
  (if (Variables|/Game/Blueprints/BP_Blueprint/BP_WorldObjects/BP_NPC_Prototype.BP_NPC_Prototype_C|GetSecondCard _asbp_npc_prototype)
    (return true)
    (else
      (return false))))

(fn LooseGame)

(fn WinGame)