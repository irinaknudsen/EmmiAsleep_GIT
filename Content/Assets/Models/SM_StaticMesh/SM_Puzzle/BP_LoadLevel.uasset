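; BP_LoadLevel is a level exit trigger that moves the player to the OutsidePlaceHolder level.
; It caches the BP_Emmi player pawn on BeginPlay, then on Tick waits until the PinchManager's current level reaches at least six.
; Once that holds and BP_Emmi overlaps its collision component, it opens the level a single time through a DoOnce.
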(event EventTick
  (params (DeltaSeconds :type Float%20%28single-precision%29))
  (if (>= (Variables|/Game/Blueprints/BP_Blueprint/BP_Player/BP_PinchManager.BP_PinchManager_C|GetcurrentLevel (Variables|/Game/Blueprints/BP_Blueprint/BP_Player/BP_Emmi.BP_Emmi_C|GetPinchManager (Variables|Default|Getplayer))) 6)
    (if (> (Utilities|Array|Length (Collision|GetOverlappingActors (Variables|Default|GetCollisionComponent) "/Game/Blueprints/BP_Blueprint/BP_Player/BP_Emmi.BP_Emmi_C" :!class /Script/Engine.PrimitiveComponent)) 0)
      (Utilities|FlowControl|DoOnce false
        (:Completed
          (Game|OpenLevel(byName) "OutsidePlaceHolder"))))))

(event EventBeginPlay
  (bind _asbp_emmi (Utilities|Casting|CastToBP_Emmi (Game|Player|GetPlayerPawn 0)))
  (Variables|Default|Setplayer _asbp_emmi))

(fn ConstructionScript)